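; Spawner actor that stacks random floor actors into an ongoing vertical level as the player climbs.
; On BeginPlay it spawns a first floor and caches the player, then each Tick spawns another whenever the player rises above the newest floor's origin height.
; Each floor class comes randomly from one of four lists selected by SkyGameMode's difficulty, and attaches at the previous floor's EndPoint location.
; The K key forces a spawn.
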(event `Key|K`
  (params (Key :type "Key Structure" :default "AnyKey"))
  (:`Pressed`
    (`KismetSystemLibrary.PrintString` "Spawning new floor")
    (`self.SpawnFloor`)))

(event `self.ReceiveBeginPlay`
  (`|ExecutionSequence`
    (:`then_0`
      (`self.BeginFloorSpawning`))
    (:`then_1`
      (bind _asplayer (cast `/Game/Blueprints/Actors/Characters/Player` (`Controller.K2_GetPawn` (`GameplayStatics.GetPlayerController` 0))))
      (set `self.Player` _asplayer))))

(event `self.ReceiveActorBeginOverlap`
  (params (OtherActor :type "Actor Object Reference")))

(event `self.ReceiveTick`
  (params (DeltaSeconds :type "Float (single-precision)"))
  (`self.Try to Spawn`))

(fn `BeginFloorSpawning`
  (`self.SpawnFloor`))

(fn `GetDificulty`
  (returns (dificulty :type Integer))
  (bind _assky_game_mode (cast `/Game/Blueprints/SkyGameMode` (`GameplayStatics.GetGameMode`)))
  (return (`/Game/Blueprints/SkyGameMode.dificulty` _assky_game_mode)))

(fn `GetListofFloorsFromDificulty`
  (returns (ListofFloors :type "Array of /Game/Blueprints/Actors/Floors/Floor Class Reference"))
  (bind _dificulty (`self.GetDificulty`))
  (switch `int` _dificulty
    (:`0`
      (return (`self.ListofFloors_0`)))
    (:`1`
      (return (`self.ListofFloors_1`)))
    (:`2`
      (return (`self.ListofFloors_2`)))
    (:`3`
      (return (`self.ListofFloors_3`)))))

(fn `GetRandomFloor`
  (returns (Item :type "/Game/Blueprints/Actors/Floors/Floor Class Reference"))
  (bind _listoffloors (`self.GetListofFloorsFromDificulty`))
  (bind _result (`/Engine/EditorBlueprintResources/StandardMacros.DecrementInt` (`KismetArrayLibrary.Array_Length` _listoffloors))
    (:`  `
      (return (`KismetArrayLibrary.Array_Get` _listoffloors (`KismetMathLibrary.RandomInteger` _result))))))

(fn `SpawnFloor`
  (bind _lastfloor (`self.LastFloor`))
  (bind _returnvalue_location (`KismetMathLibrary.BreakTransform` (`SceneComponent.K2_GetComponentToWorld` (`/Game/Blueprints/Actors/Floors/Floor.EndPoint` (`self.LastFloor`)))))
  (`/Engine/EditorBlueprintResources/StandardMacros.IsValid` _lastfloor
    (:`Is Valid`
      (`|ExecutionSequence`
        (:`then_0`
          (set `self.LastFloor` _lastfloor))
        (:`then_1`
          (set `self.LastFloorEndPoint` _returnvalue_location))
        (:`then_2`
          (bind _item (`self.GetRandomFloor` :!label _label))
          (bind _returnvalue (`|SpawnActorFromClass` _item (`KismetMathLibrary.MakeTransform` (`self.LastFloorEndPoint`)) "Undefined" "OverrideRootScale"))
          (bind _output_get (set `self.LastFloor` _returnvalue))
          (bind (_returnvalue_x _returnvalue_y _returnvalue_z) (`KismetMathLibrary.BreakVector` (`self.K2_GetActorLocation` _output_get)))
          (set `self.LastFloorHeight` _returnvalue_z)
          (return))))
    (:`Is Not Valid`
      (goto _label))))

(fn `Try to Spawn`
  (bind (_returnvalue_x _returnvalue_y _returnvalue_z) (`KismetMathLibrary.BreakVector` (`self.K2_GetActorLocation` (`self.Player`))))
  (`|ExecutionSequence`
    (:`then_0`
      (set `self.playerheight` _returnvalue_z))
    (:`then_1`
      (if (> (`self.playerheight`) (`self.LastFloorHeight`))
        (`self.SpawnFloor`)))))

(fn `UserConstructionScript`)