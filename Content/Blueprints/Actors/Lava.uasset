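; Lava is a rising hazard that climbs along world Z and kills the player on contact.
; After a start delay it plays an attached fire sound, sets a base speed and starts a looping timer that increases it in steps.
; Tick feeds that speed into movement input.
; A mesh overlap with the player halts the lava, clears the timer and triggers death through the SkyController.
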(event `self.ReceiveBeginPlay`
  (`KismetSystemLibrary.K2_SetTimer` null "Start" (`self.starttime`)))

(event `self.ReceiveActorBeginOverlap`
  (params (OtherActor :type "Actor Object Reference")))

(event `self.ReceiveTick`
  (params (DeltaSeconds :type "Float (single-precision)"))
  (`self.AddMovementInput` (`KismetMathLibrary.MakeVector` 0.0 0.0 (`self.speed`))))

(event `self.MeshComponent.OnComponentBeginOverlap`
  (params (OtherActor :type "Actor Object Reference") (OtherComp :type "PrimitiveComponent Object Reference") (OtherBodyIndex :type Integer) (bFromSweep :type Boolean) (SweepResult :type "HitResult Structure (by ref)"))
  (bind _asplayer (cast `/Game/Blueprints/Actors/Characters/Player` OtherActor))
  (`self.LavaHitPlayer` _asplayer))

(fn `incspeed`
  (set `self.speed` (+ (`self.speed`) (`self.speedincrement`))))

(fn `LavaHitPlayer`
  (params (other :type "/Game/Blueprints/Actors/Characters/Player Object Reference"))
  (`|ExecutionSequence`
    (:`then_0`
      (`self.Stop`))
    (:`then_1`
      (bind _assky_controller (cast `/Game/Blueprints/SkyController` (`self.GetController` other)))
      (`/Game/Blueprints/SkyController.Die` _assky_controller)
      (return))))

(fn `Start`
  (`|ExecutionSequence`
    (:`then_0`
      (`GameplayStatics.SpawnSoundAttached` "/Game/StarterContent/Audio/Fire01.Fire01" (`self.CollisionComponent`) "None" (0.0 0.0 0.0) (struct) "KeepRelativeOffset" false 0.2))
    (:`then_1`
      (set `self.speed` 0.05))
    (:`then_2`
      (bind _returnvalue (`KismetSystemLibrary.K2_SetTimer` null "incspeed" (`self.timeinterval`) true))
      (set `self.timerhandle` _returnvalue))))

(fn `Stop`
  (set `self.speed` 0.0)
  (`KismetSystemLibrary.K2_ClearTimerHandle` (`self.timerhandle`))
  (return))

(fn `UserConstructionScript`)