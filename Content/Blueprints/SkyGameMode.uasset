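; SkyGameMode tracks the player's score and difficulty in what appears to be a vertical climbing game.
; Each Tick with a valid Player, Score rises to the truncated height in meters while the SkyController reports IsAlive, so it records the peak.
; A switch on the stringified Score selects tiers at exact milestone values, and Dificulty only ever increases.
; Collapsed graphs split each step.
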(event EventBeginPlay)

(event EventTick
  (params (DeltaSeconds :type Float%20%28single-precision%29))
  (Utilities|IsValid (Variables|Default|Getplayer)
    (:Is%20Valid
      (Utilities|FlowControl|Sequence
        (:then_0
          (CallFunction|SetScore))
        (:then_1
          (CallFunction|SetDificulty))))))

(fn ConstructionScript)

(fn SetScore
  (Utilities|FlowControl|Sequence
    (:then_0
      (|SetPlayerHeight))
    (:then_1
      (|ifPlayerHeight>Score
        (:then
          (|IfPlayerisAlive)
          (Variables|Default|SetScore (Math|Float|Truncate (LocalVariables|GetPlayerHeight))))
        (:else
          _))
      (return))))

(fn SetDificulty
  (Utilities|FlowControl|Sequence
    (:then_0
      (|SetNewDificultyfromScore))
    (:then_1
      (|IncreaseDificultyifNewDificultyishigher))))